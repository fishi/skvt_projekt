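; Base NPC character with health, punch melee, sight detection and a takedown interaction supplied through ability and input-context getters.
; Damage feeds the Health component and plays a hit montage, while death ragdolls the mesh and sets a five-second lifespan.
; Sightings flag the player as seen on the cached AI controller.
; Nav-link jumps launch the capsule along a suggested projectile arc, with debug drawing and leftover unwired arc math.
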(event Died(Health)
  (CallFunction|TriggerDeath))

(event OnSeePawn(PawnSensing)
  (params (Pawn :type Pawn%20Object%20Reference))
  (Default|SetPlayerSeen (Variables|Default|GetBaseControllerRef) true))

(event EventJumpingNavLinkReached
  (params (JumpDestination :type Vector :default "0, 0, 0"))
  (bind _worldlocation (CallFunction|GetTeleportDestination JumpDestination))
  (if (CallFunction|IsHigherThanCurrentPosition _worldlocation)
    _
    (else
      _))
  (CallFunction|Jumpto _worldlocation))

(event Collision|EventActorBeginOverlap
  (params (OtherActor :type Actor%20Object%20Reference)))

(event EventTick
  (params (DeltaSeconds :type Float%20%28single-precision%29)))

(event EventPossessed
  (params (NewController :type Controller%20Object%20Reference))
  (CallFunction|InitController NewController))

(event Game|Damage|EventAnyDamage
  (params (Damage :type Float%20%28single-precision%29) (DamageType :type Damage%20Type%20Object%20Reference) (InstigatedBy :type Controller%20Object%20Reference) (DamageCauser :type Actor%20Object%20Reference))
  (Default|ProcessDamage (Variables|Default|GetHealth) Damage)
  (Animation|PlayAnimMontage "/Game/Skvt/Characters/Animations/Attacks/AM_Hit_punch.AM_Hit_punch" 1.0 "None"))

(fn ConstructionScript)

(fn TriggerDeath
  (Physics|SetSimulatePhysics (Variables|Character|GetMesh) true)
  (Pawn|Components|CharacterMovement|DisableMovement (Variables|Character|GetCharacterMovement))
  (Actor|SetLifeSpan 5.0))

(fn InitController
  (params (Object :type Object%20Object%20Reference))
  (bind _asaic_base_controller (Utilities|Casting|CastToAIC_BaseController Object))
  (Variables|Default|SetBaseControllerRef _asaic_base_controller))

(fn DoMeleeAttack
  (Default|Attack (Variables|Default|GetMeleeAttack) (Transformation|GetWorldLocation (Variables|Default|GetMeleeTraceStart)) (Transformation|GetWorldLocation (Variables|Default|GetMeleeTraceEnd)))
  (bind _returnvalue (Animation|PlayAnimMontage "/Game/Skvt/Characters/Animations/Attacks/AM_Att_punch.AM_Att_punch" 1.0 "None"))
  (return _returnvalue))

(fn GetTeleportDestination
  (params (CapsuleBottom :type Vector))
  (return (+ CapsuleBottom (* (Math|Vector|VectorUp) (Components|Capsule|GetScaledCapsuleHalfHeight (Variables|Collision|GetCapsuleComponent))))))

(fn IsHigherThanCurrentPosition
  (params (OtherPosition :type Vector%203f%20Structure))
  (return (> (.Z (Class|KismetMathLibrary|BreakVector3f OtherPosition)) (.Z (Class|KismetMathLibrary|BreakVector3f (Transformation|GetActorLocation))))))

(fn Jumpto
  (params (DestLocation :type Vector))
  (bind _returnvalue (Transformation|GetActorLocation))
  (bind _capsulecomponent (Variables|Collision|GetCapsuleComponent))
  (bind _returnvalue_2 (Transformation|GetWorldRotation _capsulecomponent))
  (bind (_roll _pitch) (Math|Rotator|BreakRotator _returnvalue_2))
  (bind _output_get (LocalVariables|SetDest DestLocation))
  (Utilities|FlowControl|Sequence
    (:then_0
      (if (< (.Z (Math|Vector|BreakVector (LocalVariables|GetDest))) (.Z (Math|Vector|BreakVector (Transformation|GetActorLocation))))
        (LocalVariables|SetToUp (Math|Vector|VectorUp))
        (LocalVariables|SetToDest (Math|Vector|Normalize (- (LocalVariables|GetDest) (Transformation|GetActorLocation))))
        (LocalVariables|SetToForward (Math|Vector|Normalize (Math|Vector|MakeVector (.X (Math|Vector|BreakVector (LocalVariables|GetDest))) (.Y (Math|Vector|BreakVector (LocalVariables|GetDest))) (.Z (Math|Vector|BreakVector (Transformation|GetActorLocation))))))
        (bind _output_get_2 (LocalVariables|SetAngleToDest (Class|KismetMathLibrary|QuatGetAngle (Class|KismetMathLibrary|QuatFindBetweenVectors (LocalVariables|GetToUp) (LocalVariables|GetToDest)))))
        (bind _output_get_3 (LocalVariables|SetHalfAngleToForward (* (Class|KismetMathLibrary|QuatGetAngle (Class|KismetMathLibrary|QuatFindBetweenVectors (LocalVariables|GetToUp) (LocalVariables|GetToForward))) 0.5)))))
    (:then_1
      (bind _outlaunchvelocity (Game|SuggestProjectileVelocityCustomArc (Transformation|GetActorLocation) _output_get 0.0 (LocalVariables|GetJumpArc)))
      (Character|LaunchCharacter _outlaunchvelocity true true)
      (Transformation|SetWorldRotation _capsulecomponent (Math|Rotator|MakeRotator _roll _pitch (.Yaw (Math|Rotator|BreakRotator (Math|Rotator|FindLookatRotation (Transformation|GetActorLocation) (LocalVariables|GetDest))))) false false)
      (Rendering|Debug|DrawDebugArrow _returnvalue (+ (* (Math|Vector|Normalize _outlaunchvelocity) 1e+02) _returnvalue) 0.0 "(R=0.843726,G=0.000000,B=1.000000,A=1.000000)" 1e+01 0.0)
      (Rendering|Debug|DrawDebugSphere (LocalVariables|GetApex) 1e+01 12 "(R=1.000000,G=1.000000,B=1.000000,A=1.000000)" 1e+01)
      (Rendering|Debug|DrawDebugSphere (LocalVariables|GetDest) 1e+01 12 "(R=1.000000,G=0.000000,B=0.000000,A=1.000000)" 1.0)
      (Development|PrintString (Utilities|String|ToString(Float) (LocalVariables|GetJumpArc))))))

(fn CalculateJumpDuration
  (params (HorizontalDistance :type Float%20%28double-precision%29))
  (return (Math|Float|Max(Float) (/ HorizontalDistance (Class|MovementComponent|GetMaxSpeed (Variables|Character|GetCharacterMovement))) (Variables|Default|GetMinJumpDuration))))

(fn GetInputMappingContext
  (return "/Game/Skvt/Characters/Input/IMC_EnemyNPCInteraction.IMC_EnemyNPCInteraction"))

(fn GetInteractiveAbilities
  (return (Utilities|Array|MakeArray "/Game/Skvt/Blueprints/BPC_TakedownAbility.BPC_TakedownAbility_C")))