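; Player controller for Skvt that handles Enhanced Input setup, HUD lifetime on possession changes, a pausing main menu, and swapping to a random known pawn.
; Each tick it sphere-traces between the character's melee trace points for a BPI_Interactive actor.
; When that target changes, it swaps in the target's input mapping context, rebuilds the pawn's interactive ability components from classes the target supplies, and shows them on the HUD.
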(event Custom|OnResumeRequested
  ;[0.01096 0.01161 0.0137] Ingame menu and Pausing
  (CallFunction|ResumeGame))

(event Input|EnhancedActionEvents|EnhancedInputActionIA_Swap
  (params (ActionValue :type Boolean) (ElapsedSeconds :type Float%20%28double-precision%29) (TriggeredSeconds :type Float%20%28double-precision%29) (InputAction :type Input%20Action%20Object%20Reference :default "/Game/Skvt/Characters/Input/Actions/IA_Swap.IA_Swap"))
  (:Triggered
    (CallFunction|SwapPawn)))

(event Input|EnhancedActionEvents|EnhancedInputActionIA_OpenMenu
  (params (ActionValue :type Boolean) (ElapsedSeconds :type Float%20%28double-precision%29) (TriggeredSeconds :type Float%20%28double-precision%29) (InputAction :type Input%20Action%20Object%20Reference :default "/Game/Skvt/Characters/Input/Actions/IA_OpenMenu.IA_OpenMenu"))
  ;[0.01096 0.01161 0.0137] Ingame menu and Pausing
  (:Triggered
    (bind _mainmenu (CallFunction|ToggleGamePause))
    (Utilities|IsValid _mainmenu
      (:Is%20Valid
        (EventDispatchers|AssignOnResumeRequested _mainmenu (delegate Custom|OnResumeRequested))))))

(event EventBeginPlay
  (CallFunction|InitInput)
  (CallFunction|InitGameMode))

(event EventPossess
  (params (PossessedPawn :type Pawn%20Object%20Reference))
  (CallFunction|InitPlayerHUD))

(event EventUnPossess
  (params (UnpossessedPawn :type Pawn%20Object%20Reference))
  (Class|BPIInteractingActor|DestroyInteractiveAbilities(Message) UnpossessedPawn)
  (CallFunction|DeInitPlayerHUD))

(event EventTick
  (params (DeltaSeconds :type Float%20%28single-precision%29))
  (Utilities|UpdateInteractiveActor
    (:Actor%20Changed
      (CallFunction|UpdatePawnInteractiveAbilities))))

(fn ConstructionScript)

(fn InitGameMode
  (bind _asbp_skvt_game_mode (Utilities|Casting|CastToBP_SkvtGameMode (Game|GetGameMode)))
  (Variables|Default|SetSkvtGameMode _asbp_skvt_game_mode))

(fn InitInput
  (bind _self self)
  (bind _returnvalue (PlayerController|LocalPlayerSubsystems|GetEnhancedInputLocalPlayerSubsystem _self))
  (Utilities|IsValid _returnvalue
    (:Is%20Valid
      (Class|EnhancedInputSubsystemInterface|AddPlayerMappableConfig _returnvalue "/Game/Skvt/Characters/Input/PMI_SkvtMapping.PMI_SkvtMapping" "(bIgnoreAllPressedKeysUntilRelease=True,bForceImmediately=False)"))))

(fn ToggleGamePause
  (Utilities|IsValid (Variables|Default|GetMainMenu)
    (:Is%20Valid
      (CallFunction|OnResumeRequested))
    (:Is%20Not%20Valid
      (CallFunction|PauseGame)))
  (return (Variables|Default|GetMainMenu)))

(fn ResumeGame
  (Utilities|FlowControl|Sequence
    (:then_0
      (Widget|RemovefromParent (Variables|Default|GetMainMenu))
      (Variables|Default|SetMainMenu 0))
    (:then_1
      (Input|SetInputModeGameOnly self false)
      (Variables|Default|SetbShowMouseCursor false))
    (:then_2
      (Game|SetGamePaused false))))

(fn PauseGame
  (Utilities|FlowControl|Sequence
    (:then_0
      (Game|SetGamePaused true))
    (:then_1
      (Input|SetInputModeGameandUI self 0 "DoNotLock" true false)
      (Variables|Default|SetbShowMouseCursor true))
    (:then_2
      (bind _returnvalue (UserInterface|CreateWidget "/Game/Skvt/UI/Widgets/Menu/WBP_MainMenu.WBP_MainMenu_C" self))
      (bind _output_get (Variables|Default|SetMainMenu _returnvalue))
      (UserInterface|Viewport|AddtoPlayerScreen _output_get))))

(fn SwapPawn
  (Utilities|FlowControl|Sequence
    (:then_0
      (if (Utilities|Array|IsEmpty (Variables|Default|GetKnownPawns))
        (bind _outactors (Actor|GetAllActorsOfClass "/Script/Engine.Pawn"))
        (Variables|Default|SetKnownPawns _outactors)))
    (:then_1
      (Utilities|Array|RemoveItem (Variables|Default|GetKnownPawns) (Pawn|GetControlledPawn) :!label _label))
    (:then_2
      (Pawn|Possess (.OutItem (Utilities|Array|Random (Variables|Default|GetKnownPawns))))
      (goto _label))))

(fn DeInitPlayerHUD
  (Utilities|IsValid (Variables|Default|GetPlayerHUD)
    (:Is%20Valid
      (Widget|RemovefromParent (Variables|Default|GetPlayerHUD))
      (Variables|Default|SetPlayerHUD 0))))

(fn InitPlayerHUD
  (bind _returnvalue (UserInterface|CreateWidget "/Game/Skvt/UI/Widgets/WBP_PlayerHUD.WBP_PlayerHUD_C" self))
  (bind _output_get (Variables|Default|SetPlayerHUD _returnvalue))
  (UserInterface|Viewport|AddtoViewport _output_get 0))

(fn FindInteractiveActor
  (bind _asbp_skvt_base_char (Utilities|Casting|CastToBP_SkvtBaseChar (Pawn|GetControlledPawn))
    (:then
      (bind (_outhit _returnvalue) (Collision|SphereTraceByChannel (Transformation|GetWorldLocation (Variables|/Game/Skvt/Characters/BP_SkvtBaseChar.BP_SkvtBaseChar_C|GetMeleeAttackTraceStart _asbp_skvt_base_char)) (Transformation|GetWorldLocation (Variables|/Game/Skvt/Characters/BP_SkvtBaseChar.BP_SkvtBaseChar_C|GetMeleeAttackTraceEnd _asbp_skvt_base_char)) 6e+01 "TraceTypeQuery5" false (Utilities|Array|MakeArray (Pawn|GetControlledPawn)) "None"))
      (if _returnvalue
        (Utilities|Casting|CastToBPI_Interactive (.HitActor (Collision|BreakHitResult _outhit))
          (:then
            (return (.HitActor (Collision|BreakHitResult _outhit))))
          (:CastFailed
            (return 0)))
        (else
          (return 0))))
    (:CastFailed
      (return 0))))

(fn UpdatePawnInteractiveAbilities
  (Class|BPIInteractingActor|DestroyInteractiveAbilities(Message) (Pawn|GetControlledPawn))
  (Utilities|FlowControl|Sequence
    (:then_0
      ;[0.01096 0.01161 0.0137] Update components
      (bind _interactiveabilities (Class|BPIInteractive|GetInteractiveAbilities(Message) (Variables|Default|GetInteractiveActor)))
      (for _array_element _interactiveabilities
        (Game|AddComponentbyClass (Pawn|GetControlledPawn) _array_element (Variables|Default|GetInteractiveActor))))
    (:then_1
      ;[0.01096 0.01161 0.0137] Update HUD
      (Default|SetInteractiveAbilities (Variables|Default|GetPlayerHUD) (Actor|GetComponentsByClass (Pawn|GetControlledPawn) "/Game/Skvt/Blueprints/BPC_InteractiveAbility.BPC_InteractiveAbility_C")))))

(fn ClearInteractiveActor
  (bind _imc (Class|BPIInteractive|GetInputMappingContext(Message) (Variables|Default|GetInteractiveActor)))
  (Input|RemoveMappingContext (PlayerController|LocalPlayerSubsystems|GetEnhancedInputLocalPlayerSubsystem self) _imc "(bIgnoreAllPressedKeysUntilRelease=True,bForceImmediately=False)")
  (Variables|Default|SetInteractiveActor 0)
  (CallFunction|UpdatePawnInteractiveAbilities))