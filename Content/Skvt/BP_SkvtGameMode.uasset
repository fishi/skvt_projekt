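; Game mode that coordinates highlighting and EMP effects on electronic devices around a given pawn.
; Highlight enable and EMP trigger both gather devices within a fixed radius of the pawn via FindElectronicDevices, then message each one.
; Highlight disable instead clears every BPI_ElectronicDevice actor in the world and also runs on BeginPlay, so play starts with highlights off.
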(event EventBeginPlay
  (CallFunction|DisableElectronicHighlight))

(fn ConstructionScript)

(fn EnableElectronicHighlight
  (params (Pawn :type Pawn%20Object%20Reference))
  (bind _devices (CallFunction|FindElectronicDevices (Transformation|GetActorLocation Pawn) 5e+02))
  (for _array_element _devices
    (Class|BPIElectronicDevice|SetHighlighted(Message) _array_element true)))

(fn DisableElectronicHighlight
  (bind _outactors (Actor|GetAllActorswithInterface "/Game/Skvt/Blueprints/BPI_ElectronicDevice.BPI_ElectronicDevice_C"))
  (for _array_element _outactors
    (Class|BPIElectronicDevice|SetHighlighted(Message) _array_element false)))

(fn TriggerEMP
  (params (Pawn :type Pawn%20Object%20Reference))
  (bind _devices (CallFunction|FindElectronicDevices (Transformation|GetActorLocation Pawn) 5e+02))
  (for _array_element _devices
    (Class|BPIElectronicDevice|ReceiveEMP(Message) _array_element)))