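; Takedown ability component that lets its owner silently finish a target actor from behind, with a "Take down" interaction prompt.
; BeginPlay caches the owner's movement and mesh components and the target's BPC_Health.
; IA_Takedown requires the owner to be crouched, the target alive and both facing similar directions via a forward-vector dot product.
; It then plays a punch montage and applies heavy damage to the target when it completes.
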(event Input|EnhancedActionEvents|EnhancedInputActionIA_Takedown
  (params (ActionValue :type Boolean) (ElapsedSeconds :type Float%20%28double-precision%29) (TriggeredSeconds :type Float%20%28double-precision%29) (InputAction :type Input%20Action%20Object%20Reference :default "/Game/Skvt/Characters/Input/Actions/IA_Takedown.IA_Takedown"))
  (:Triggered
    (if (CallFunction|CanInteractwithControlledPawn)
      (Animation|Montage|PlayMontage (Variables|Default|GetMeshComponentRef) "/Game/Skvt/Characters/Animations/Attacks/AM_Att_punch.AM_Att_punch"
        (:OnCompleted
          (Game|Damage|ApplyDamage (Variables|Default|GetTargetActor) 1e+03 0 0))))))

(event EventBeginPlay
  (CallFunction|InitMovementComponent)
  (CallFunction|InitMeshComponent)
  (CallFunction|InitHealthComponent))

(event EventTick
  (params (DeltaSeconds :type Float%20%28single-precision%29))
  (|CallParentFunction DeltaSeconds) ; This node is disabled and will not be called.\nDrag off pins to build functionality.
)

(fn CanInteractwithControlledPawn
  (bind _movementcomponentref (Variables|Default|GetMovementComponentRef))
  (bind _targethealthcomponentref (Variables|Default|GetTargetHealthComponentRef))
  (Utilities|IsValid _targethealthcomponentref
    (:Is%20Valid
      (Utilities|IsValid _movementcomponentref
        (:Is%20Valid
          (return (Math|Boolean|ANDBoolean (AI|Components|NavMovement|IsCrouching _movementcomponentref) (> (Math|Vector|DotProduct (Transformation|GetActorForwardVector (Components|GetOwner)) (Transformation|GetActorForwardVector (Variables|Default|GetTargetActor))) 0.3) (not (Default|IsDead _targethealthcomponentref)))))
        (:Is%20Not%20Valid
          (return false))))
    (:Is%20Not%20Valid
      (return false))))

(fn InitMovementComponent
  (Variables|Default|SetMovementComponentRef (Actor|GetComponentbyClass (Components|GetOwner) "/Script/Engine.CharacterMovementComponent")))

(fn InitHealthComponent
  (Variables|Default|SetTargetHealthComponentRef (Actor|GetComponentbyClass (Variables|Default|GetTargetActor) "/Game/Skvt/Blueprints/BPC_Health.BPC_Health_C")))

(fn InitMeshComponent
  (Variables|Default|SetMeshComponentRef (Actor|GetComponentbyClass (Components|GetOwner) "/Script/Engine.SkeletalMeshComponent")))

(fn GetInteractionPrompt
  (return "Take down"))