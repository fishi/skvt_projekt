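; BPC_Health is a health component Blueprint that tracks damage and death for its owner.
; On BeginPlay it replaces a non-positive MaxHealth with a default, then fills Health to that maximum.
; ProcessDamage subtracts damage without clamping and calls the Died dispatcher whenever Health is at or below zero, including on repeat hits.
; GetHealthPercent returns a clamped health fraction, and Tick is unused.
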(event EventBeginPlay
  (CallFunction|InitHealth))

(event EventTick
  (params (DeltaSeconds :type Float%20%28single-precision%29)))

(fn ProcessDamage
  (params (Damage :type Float%20%28double-precision%29))
  (Variables|Default|SetHealth (- (Variables|Default|GetHealth) Damage))
  (if (CallFunction|IsDead)
    (Default|CallDied)))

(fn IsDead
  (return (<= (Variables|Default|GetHealth) 0.0)))

(fn GetHealthPercent
  (return (Math|Float|Clamp(Float) (/ (Variables|Default|GetHealth) (Variables|Default|GetMaxHealth)))))

(fn InitHealth
  (Utilities|FlowControl|Sequence
    (:then_0
      ;[0.01096 0.01161 0.0137] Sanitize MaxHealth
      (if (<= (Variables|Default|GetMaxHealth) 0.0)
        (Variables|Default|SetMaxHealth 1e+02)))
    (:then_1
      ;[0.01096 0.01161 0.0137] Reset Health to MaxHealth
      (Variables|Default|SetHealth (Variables|Default|GetMaxHealth)))))