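; BP_SkvtScreen is a screen actor that shows a WBP_SkvtWeb widget through its Webpage component and supports a highlighted state.
; On BeginPlay, Initialize casts the component's widget to WBP_SkvtWeb and caches it in WebpageRef.
; SetHighlighted swaps visibility between the two components: highlighting shows the StaticMesh and hides the Webpage, and clearing it does the reverse, without propagating to children.
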(event EventBeginPlay
  (CallFunction|Initialize))

(event Collision|EventActorBeginOverlap
  (params (OtherActor :type Actor%20Object%20Reference)))

(event EventTick
  (params (DeltaSeconds :type Float%20%28single-precision%29)))

(event EventSetHighlighted
  (params (Highlighted :type Boolean))
  (Rendering|SetVisibility (Variables|Default|GetStaticMesh) Highlighted false)
  (Rendering|SetVisibility (Variables|Default|GetWebpage) (not Highlighted) false))

(fn ConstructionScript)

(fn Initialize
  (bind _aswbp_skvt_web (Utilities|Casting|CastToWBP_SkvtWeb (UserInterface|GetWidget (Variables|Default|GetWebpage))))
  (Variables|Default|SetWebpageRef _aswbp_skvt_web))