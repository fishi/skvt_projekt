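; Interactive component that lets a player controller take input control of its owning actor through start and stop interaction events.
; Starting stores the controller if none is set, enables owner input, adds an Enhanced Input mapping context and creates a HUD widget, without adding it to the viewport.
; Stopping, for that same controller, removes the context and widget but leaves owner input enabled and the controller stored.
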(event EventBeginPlay)

(event EventTick
  (params (DeltaSeconds :type Float%20%28single-precision%29)))

(event EventStartInteracting
  (params (PlayerController :type Player%20Controller%20Object%20Reference) (Pawn :type Pawn%20Object%20Reference))
  (Utilities|IsValid (Variables|Default|GetPlayerController)
    (:Is%20Not%20Valid
      (bind _output_get (Variables|Default|SetPlayerController PlayerController))
      (Input|EnableInput (Components|GetOwner) _output_get)
      (Input|AddMappingContext (PlayerController|LocalPlayerSubsystems|GetEnhancedInputLocalPlayerSubsystem (Variables|Default|GetPlayerController)) (Variables|Default|GetIMC) 1 "(bIgnoreAllPressedKeysUntilRelease=True,bForceImmediately=False)")
      (bind _returnvalue (UserInterface|CreateWidget (Variables|Default|GetHUDWidgetClass) (Variables|Default|GetPlayerController)))
      (Variables|Default|SetHUDWidget _returnvalue))))

(event EventStopInteracting
  (params (PlayerController :type Player%20Controller%20Object%20Reference) (Pawn :type Pawn%20Object%20Reference))
  (if (== PlayerController (Variables|Default|GetPlayerController))
    (Utilities|FlowControl|Sequence
      (:then_0
        (Input|RemoveMappingContext (PlayerController|LocalPlayerSubsystems|GetEnhancedInputLocalPlayerSubsystem (Variables|Default|GetPlayerController)) (Variables|Default|GetIMC) "(bIgnoreAllPressedKeysUntilRelease=True,bForceImmediately=False)"))
      (:then_1
        (Utilities|IsValid (Variables|Default|GetHUDWidget)
          (:Is%20Valid
            (Widget|RemovefromParent (Variables|Default|GetHUDWidget))
            (Variables|Default|SetHUDWidget 0)))))))