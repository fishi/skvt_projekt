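; Interaction ability component that lets the player switch a target electronic device on or off.
; On the Interact input, it toggles the target through BPI_ElectronicDevice, provided the device is not destroyed.
; The prompt reads "Turn on" or "Turn off" to match the device's current state.
; A shared GetED helper casts TargetActor to the interface, and a failed cast makes interaction unavailable.
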(event Input|EnhancedActionEvents|EnhancedInputActionIA_Interact
  (params (ActionValue :type Boolean) (ElapsedSeconds :type Float%20%28double-precision%29) (TriggeredSeconds :type Float%20%28double-precision%29) (InputAction :type Input%20Action%20Object%20Reference :default "/Game/Skvt/Characters/Input/Actions/IA_Interact.IA_Interact"))
  (:Triggered
    (if (CallFunction|CanInteractwithControlledPawn)
      (bind _asbpi_electronic_device (Utilities|GetED)
        (:then
          (Default|ToggleTurnedon _asbpi_electronic_device))))))

(event EventBeginPlay)

(event EventTick
  (params (DeltaSeconds :type Float%20%28single-precision%29)))

(fn GetInteractionPrompt
  (bind _asbpi_electronic_device (Utilities|GetED)
    (:then
      (bind _ison (Default|IsTurnedon _asbpi_electronic_device))
      (if _ison
        (return "Turn off")
        (else
          (return "Turn on"))))))

(fn CanInteractwithControlledPawn
  (bind _asbpi_electronic_device (Utilities|GetED)
    (:then
      (bind _isdestroyed (Default|IsDestroyed _asbpi_electronic_device))
      (return (not _isdestroyed)))
    (:CastFailed
      (return false))))