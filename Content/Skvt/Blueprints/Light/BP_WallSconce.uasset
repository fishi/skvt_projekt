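; BP_WallSconce is a wall sconce light with configurable brightness, color, cone angles and lit state.
; UpdateLight pushes those variables onto the SconceLight component, using its visibility for on and off.
; The construction script calls UpdateLight, so the light reflects its settings when constructed.
; ToggleLight and SetLit change IsLit and then reapply everything through the same function.
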(fn ConstructionScript
  (CallFunction|UpdateLight))

(fn UpdateLight
  (bind _sconcelight (Variables|Default|GetSconceLight))
  (Rendering|Components|Light|SetIntensity _sconcelight (Variables|Light|GetBrightness))
  (Rendering|Components|Light|SetLightColor _sconcelight (Variables|Light|GetColor) true)
  (Rendering|Lighting|SetInnerConeAngle _sconcelight (Variables|Light|GetInner%20Cone%20Angle))
  (Rendering|Lighting|SetOuterConeAngle _sconcelight (Variables|Light|GetOuter%20Cone%20Angle))
  (Rendering|SetVisibility _sconcelight (Variables|Light|GetIs%20Lit) false))

(fn ToggleLight
  (Variables|Light|SetIs%20Lit (not (Variables|Light|GetIs%20Lit)))
  (CallFunction|UpdateLight))

(fn SetLit
  (params (Lit :type Boolean))
  (Variables|Light|SetIs%20Lit Lit)
  (CallFunction|UpdateLight))