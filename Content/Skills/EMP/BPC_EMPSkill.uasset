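; EMP skill component that lets its owning Character trigger an EMP.
; On BeginPlay it caches the owner as a Character and the current game mode as BP_SkvtGameMode.
; The FireEMP event delegates to the game mode's TriggerEMP, passing the Character, so the component holds no effect logic itself.
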(event Custom|FireEMP
  (Default|TriggerEMP (Variables|Default|GetGameMode) (Variables|Default|GetCharacter)))

(event EventBeginPlay
  (CallFunction|InitCharacter)
  (CallFunction|InitGameMode))

(event EventTick
  (params (DeltaSeconds :type Float%20%28single-precision%29)))

(fn InitCharacter
  (bind _ascharacter (Utilities|Casting|CastToCharacter (Components|GetOwner)))
  (Variables|Default|SetCharacter _ascharacter))

(fn InitGameMode
  (bind _asbp_skvt_game_mode (Utilities|Casting|CastToBP_SkvtGameMode (Game|GetGameMode)))
  (Variables|Default|SetGameMode _asbp_skvt_game_mode))