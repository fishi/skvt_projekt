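; Actor component that gives its owning Character an EMP ability to hit nearby electronic devices.
; On BeginPlay it caches the owner as a Character and the current BP_SkvtGameMode.
; The IA_TriggerEMP input action fires the EMP, which finds electronic devices within EMPRadius of the character's location.
; Each device found receives the EMP through an interface message, leaving the reaction to the device.
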(event Input|EnhancedActionEvents|EnhancedInputActionIA_TriggerEMP
  (params (ActionValue :type Boolean) (ElapsedSeconds :type Float%20%28double-precision%29) (TriggeredSeconds :type Float%20%28double-precision%29) (InputAction :type Input%20Action%20Object%20Reference :default "/Game/Skvt/Characters/Input/Actions/IA_TriggerEMP.IA_TriggerEMP"))
  (:Triggered
    (CallFunction|FireEMP)))

(event EventBeginPlay
  (CallFunction|InitCharacter)
  (CallFunction|InitGameMode))

(fn InitCharacter
  (bind _ascharacter (Utilities|Casting|CastToCharacter (Components|GetOwner)))
  (Variables|Default|SetCharacter _ascharacter))

(fn InitGameMode
  (bind _asbp_skvt_game_mode (Utilities|Casting|CastToBP_SkvtGameMode (Game|GetGameMode)))
  (Variables|Default|SetGameMode _asbp_skvt_game_mode))

(fn FireEMP
  ;[0.01096 0.01161 0.0137] Find electronic devices around component owner
  (bind _devices (CallFunction|FindElectronicDevices (Transformation|GetActorLocation (Variables|Default|GetCharacter)) (Variables|Default|GetEMPRadius)))
  ;[0.01096 0.01161 0.0137] Message them to receive EMP via interface
  (for _array_element _devices
    (Class|BPIElectronicDevice|ReceiveEMP(Message) _array_element)))